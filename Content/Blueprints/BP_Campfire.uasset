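; Campfire checkpoint actor for the side-scroller character.
; When BP_SideScrollerCharacter enters the trigger box, it sets that character's checkpoint to the respawn point's world location, restores full health and registers itself as the nearby campfire.
; Leaving the trigger clears the nearby campfire reference, and a debug message prints on entry.
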(event `self.Triggerbox.OnComponentBeginOverlap`
  (params (OverlappedComponent :type "PrimitiveComponent Object Reference") (OtherActor :type "Actor Object Reference") (OtherComp :type "PrimitiveComponent Object Reference") (OtherBodyIndex :type Integer) (bFromSweep :type Boolean) (SweepResult :type "HitResult Structure (by ref)"))
  (bind _asbp_side_scroller_character (cast `/Game/Blueprints/BP_SideScrollerCharacter` OtherActor))
  (`KismetSystemLibrary.PrintString` "CHECKPOINT 1")
  (`/Game/Blueprints/BP_SideScrollerCharacter.SetCheckPoint` _asbp_side_scroller_character (`SceneComponent.K2_GetComponentLocation` (`self.RespawnPoiint`)))
  (set `/Game/Blueprints/BP_SideScrollerCharacter.CurrentHealth` (`/Game/Blueprints/BP_SideScrollerCharacter.MaxHealth` _asbp_side_scroller_character) _asbp_side_scroller_character)
  (set `/Game/Blueprints/BP_SideScrollerCharacter.NearbyCampfire` self _asbp_side_scroller_character))

(event `self.Triggerbox.OnComponentEndOverlap`
  (params (OverlappedComponent :type "PrimitiveComponent Object Reference") (OtherActor :type "Actor Object Reference") (OtherComp :type "PrimitiveComponent Object Reference") (OtherBodyIndex :type Integer))
  (bind _asbp_side_scroller_character (cast `/Game/Blueprints/BP_SideScrollerCharacter` OtherActor))
  (set `/Game/Blueprints/BP_SideScrollerCharacter.NearbyCampfire` null _asbp_side_scroller_character))

(fn `UserConstructionScript`)