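; Flying bird enemy for the side-scroller that chases the player and attacks up close.
; Tick moves it on the XZ plane without sweep while the player is between stop and detection range, mirroring the flipbook via X scale.
; Near the stop distance, it plays an attack flipbook, applies delayed damage without rechecking range, then resumes the flying animation.
; CanAttack and a cooldown timer gate repeat attacks.
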(event `self.ReceiveBeginPlay`
  (`parent.ReceiveBeginPlay`)
  (bind _asbp_side_scroller_character (cast `/Game/Blueprints/BP_SideScrollerCharacter` (`GameplayStatics.GetPlayerCharacter` 0)))
  (set `self.PlayerRef` _asbp_side_scroller_character))

(event `self.ReceiveTick`
  (params (DeltaSeconds :type "Float (single-precision)"))
  (bind _playerref (`self.PlayerRef`))
  (bind _returnvalue (- (`self.K2_GetActorLocation` _playerref) (`self.K2_GetActorLocation` self)))
  (bind _returnvalue_2 (`KismetMathLibrary.MakeVector` (.x _returnvalue) 0.0 (.z _returnvalue)))
  (bind _returnvalue_3 (`KismetMathLibrary.VSize` _returnvalue_2))
  ; Chase AI + Flip faces
  (`parent.ReceiveTick` DeltaSeconds)
  (`/Engine/EditorBlueprintResources/StandardMacros.IsValid` _playerref
    (:`Is Valid`
      (if (and (<= _returnvalue_3 (`self.DetectionRange`)) (>= _returnvalue_3 (`self.StopDistance`)))
        (`self.K2_SetActorLocation` (+ (`self.K2_GetActorLocation` self) (* (`KismetMathLibrary.Normal` _returnvalue_2) (* (`self.ChaseSpeed`) DeltaSeconds))))
        (if (> (.x _returnvalue) 0.0)
          (`SceneComponent.SetRelativeScale3D` (`self.PaperFlipbook`) (-0.3 0.3 0.3))
          (else
            (`SceneComponent.SetRelativeScale3D` (`self.PaperFlipbook`) (0.3 0.3 0.3))))
        (elif (<= (`KismetMathLibrary.VSize` (- (`self.K2_GetActorLocation` (`self.PlayerRef`)) (`self.K2_GetActorLocation` self))) (+ (`self.StopDistance`) 50.0))
          (`KismetSystemLibrary.PrintString` "In Attack range")
          (if (and (not (`self.IsAttacking`)) (`self.CanAttack`))
            (`self.StartBirdAttack`)))))))

(event `StartBirdAttack`
  (set `self.CanAttack` false)
  (`|ExecutionSequence`
    (:`then_0`
      (set `self.IsAttacking` true)
      (`PaperFlipbookComponent.SetFlipbook` (`self.PaperFlipbook`) "/Game/PaperAssets/Enemies/BIRD_Attack-Animation.BIRD_Attack-Animation")
      (`PaperFlipbookComponent.SetLooping` (`self.PaperFlipbook`) false)
      (`PaperFlipbookComponent.PlayFromStart` (`self.PaperFlipbook`))
      (`KismetSystemLibrary.Delay` 0.35)
      (`GameplayStatics.ApplyDamage` (`self.PlayerRef`) (`self.AttackDamage`) null self)
      (`KismetSystemLibrary.Delay` 0.714)
      (set `self.IsAttacking` false)
      (`PaperFlipbookComponent.SetFlipbook` (`self.PaperFlipbook`) "/Game/PaperAssets/Enemies/BIRD_ENEMY_flyingAnimation.BIRD_ENEMY_flyingAnimation")
      (`PaperFlipbookComponent.SetLooping` (`self.PaperFlipbook`) true)
      (`PaperFlipbookComponent.PlayFromStart` (`self.PaperFlipbook`))
      (`KismetSystemLibrary.Delay` 0.72)
      (set `self.IsAttacking` false)
      (`PaperFlipbookComponent.SetFlipbook` (`self.PaperFlipbook`) "/Game/PaperAssets/Enemies/BIRD_ENEMY_flyingAnimation.BIRD_ENEMY_flyingAnimation")
      (`PaperFlipbookComponent.SetLooping` (`self.PaperFlipbook`) true)
      (`PaperFlipbookComponent.PlayFromStart` (`self.PaperFlipbook`)))
    (:`then_1`
      (`KismetSystemLibrary.K2_SetTimerDelegate` (`|CreateDelegate` :!event `ResetBirdAttack`) (`self.AttackCooldown`)))))

(event `ResetBirdAttack`
  (set `self.CanAttack` true))

(fn `UserConstructionScript`
  (`parent.UserConstructionScript`))