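; BP_Boss is a flying Lych boss enemy with a health pool and a second phase triggered by damage.
; Incoming damage is truncated to an integer and subtracted from clamped health while the boss is alive.
; Crossing the health threshold starts phase two once, playing an attack flipbook briefly before returning to the floating loop.
; The toxic cloud summon is only a debug print, and nothing here sets the death flag.
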(event `self.ReceiveBeginPlay`
  (`CharacterMovementComponent.SetMovementMode` (`self.CharacterMovement`) "MOVE_Flying" 0))

(event `TakeBossDamage`
  (params (DamageAmount :type Integer))
  (bind _sprite (`self.Sprite`))
  (bind _sprite_2 (`self.Sprite`))
  (if (not (`self.IsDead`))
    (bind _output_get (set `self.CurrentHealth` (`KismetMathLibrary.Clamp` (- (`self.CurrentHealth`) DamageAmount) 0 1000)))
    (`KismetSystemLibrary.PrintString` (`KismetStringLibrary.Conv_IntToString` _output_get))
    (if (<= (`self.CurrentHealth`) 800)
      (`/Engine/EditorBlueprintResources/StandardMacros.DoOnce` false
        (:`Completed`
          (set `self.Phase2Started` true)
          (`KismetSystemLibrary.PrintString` "Phase 2")
          (`PaperFlipbookComponent.SetFlipbook` (`self.Sprite`) "/Game/PaperAssets/FinalBoss/Lych_AttackBothHands_Animation.Lych_AttackBothHands_Animation")
          (`PaperFlipbookComponent.SetLooping` _sprite_2 false)
          (`PaperFlipbookComponent.PlayFromStart` _sprite_2)
          (`KismetSystemLibrary.PrintString` "BOSS SUMMONING TOXIC CLOUDS")
          (`KismetSystemLibrary.Delay` 1.0)
          (`PaperFlipbookComponent.SetFlipbook` (`self.Sprite`) "/Game/PaperAssets/FinalBoss/Lych_FloatingAnimation.Lych_FloatingAnimation")
          (`PaperFlipbookComponent.SetLooping` _sprite true)
          (`PaperFlipbookComponent.PlayFromStart` _sprite))))))

(event `self.ReceiveAnyDamage`
  (params (Damage :type "Float (single-precision)") (DamageType :type "DamageType Object Reference") (InstigatedBy :type "Controller Object Reference") (DamageCauser :type "Actor Object Reference"))
  (`self.TakeBossDamage` (`KismetMathLibrary.FTrunc` Damage)))

(fn `UserConstructionScript`)